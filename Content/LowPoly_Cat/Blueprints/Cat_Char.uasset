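; Playable cat character that feeds movement state to its Animation Blueprint and handles mapped look and jump input.
; Tick smooths move input, derives Turn from a mesh-to-camera dot product, and uses line traces for InAir and for blocking forward movement at obstacles.
; Jump input only sets ShouldJump, leaving the jump to TriggerJump.
; Movement mode switches between Falling and Flying by vertical velocity so OnLanded can fire.
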(event Custom|TriggerJump
  (Character|Jump))

(event Input|EnhancedActionEvents|EnhancedInputActionLook
  (params (ActionValue :type Vector%202D%20Structure) (ElapsedSeconds :type Float%20%28double-precision%29) (TriggeredSeconds :type Float%20%28double-precision%29) (InputAction :type Input%20Action%20Object%20Reference :default "/Game/LowPoly_Cat/Blueprints/Controls/Look.Look"))
  (bind _cameraboom (Variables|Default|GetCameraBoom))
  ;[1 1 1] Look Controls
  (:Triggered
    (Transformation|AddWorldRotation _cameraboom (Math|Rotator|MakeRotator 0.0 0.0 (.x ActionValue)) false false)
    (Transformation|AddRelativeRotation _cameraboom (Math|Rotator|MakeRotator 0.0 (.y ActionValue) 0.0) false false)))

(event Input|EnhancedActionEvents|EnhancedInputActionJump
  (params (ActionValue :type Boolean) (ElapsedSeconds :type Float%20%28double-precision%29) (TriggeredSeconds :type Float%20%28double-precision%29) (InputAction :type Input%20Action%20Object%20Reference :default "/Game/LowPoly_Cat/Blueprints/Controls/Jump.Jump"))
  (:Triggered
    (Variables|Default|SetshouldJump true)))

(event EventBeginPlay
  (Input|AddMappingContext (PlayerController|LocalPlayerSubsystems|GetEnhancedInputLocalPlayerSubsystem (Game|GetPlayerController 0)) "/Game/LowPoly_Cat/Blueprints/Controls/WalkRunContext.WalkRunContext" 0 "(bIgnoreAllPressedKeysUntilRelease=True,bForceImmediately=False)"))

(event Collision|EventActorBeginOverlap
  (params (OtherActor :type Actor%20Object%20Reference)))

(event EventTick
  (params (DeltaSeconds :type Float%20%28single-precision%29))
  (bind _camera (Variables|Default|GetCamera))
  (bind _returnvalue (Math|Vector|GetForwardVector _camera))
  ;[1 1 1] Set Movement Controls on Tick for AnimBP
  (Variables|Default|SetMove (Math|Float|SelectFloat (Math|Float|Clamp(Float) (Math|Float|Lerp (Variables|Default|GetMove) (.y (Input|EnhancedActionValues|GetMove)) (* DeltaSeconds (Variables|Default|GetMoveAcceleration))) -1.0 0.0) (Math|Float|Lerp (Variables|Default|GetMove) (.y (Input|EnhancedActionValues|GetMove)) (* DeltaSeconds (Variables|Default|GetMoveAcceleration))) (Variables|Default|GetCollisionAhead)))
  (Variables|Default|SetTurn (/ (Math|Vector|DotProduct (Math|Vector|GetForwardVector (Variables|Character|GetMesh)) (Math|Vector|MakeVector (.x _returnvalue) (.y _returnvalue) 0.0)) 2.0))
  ;[1 1 1] Fake Landing Test!
  (bind _returnvalue_2 (CallFunction|FakeIsFalling))
  (Variables|Default|SetinAir (not _returnvalue_2))
  (bind _returnvalue_3 (CallFunction|FakeCollisionCheck))
  (Variables|Default|SetCollisionAhead _returnvalue_3)
  ;[1 1 1] Manually switch between "Falling" and "Flying" to permit OnLanded
  (CallFunction|SwitchFallandFly))

(event EventOnLanded
  (params (Hit :type Hit%20Result%20Structure%20%28by%20ref%29))
  (Pawn|Components|CharacterMovement|SetMovementMode (Variables|Character|GetCharacterMovement) "MOVE_Flying" 0)
  (Variables|Default|SetshouldJump false))

(fn ConstructionScript)

(fn SwitchFallandFly
  (bind _charactermovement (Variables|Character|GetCharacterMovement))
  (if (< (.z (Pawn|Components|CharacterMovement|GetLastUpdateVelocity _charactermovement)) 0.0)
    (Pawn|Components|CharacterMovement|SetMovementMode _charactermovement "MOVE_Falling" 0)
    (else
      (Pawn|Components|CharacterMovement|SetMovementMode _charactermovement "MOVE_Flying" 0))))

(fn FakeIsFalling
  (bind _returnvalue (Transformation|GetActorLocation))
  (bind _returnvalue_2 (Collision|LineTraceByChannel _returnvalue (+ _returnvalue (* (Transformation|GetActorUpVector) (Math|Float|MakeLiteralFloat -9e+01))) "TraceTypeQuery1" false 0 "ForOneFrame"))
  (return _returnvalue_2))

(fn FakeCollisionCheck
  (bind _returnvalue (Transformation|GetActorLocation))
  (bind _returnvalue_2 (Collision|LineTraceByChannel _returnvalue (+ _returnvalue (* (Transformation|GetActorForwardVector) (Math|Float|MakeLiteralFloat 2.5e+02))) "TraceTypeQuery1" false 0 "ForOneFrame"))
  (return _returnvalue_2))